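; BP_Audio is an actor that switches the game's background music in response to HUD events.
; On BeginPlay it casts the player's HUD to MyHUD and binds handlers to its game start, begin move and play animation dispatchers.
; Game start deactivates the start track and plays the opening track, begin move plays the gameplay track, and the animation event plays the ending track.
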(event Custom|GameStart_Music
  (Components|Activation|Deactivate (Variables|Default|GetBGM_Start))
  (Audio|Components|Audio|Play (Variables|Default|GetBGM_OP) 0.0))

(event Custom|BeginMove_Music
  (Audio|Components|Audio|Play (Variables|Default|GetBGM_Playing) 0.0))

(event Custom|PlayED
  (Audio|Components|Audio|Play (Variables|Default|GetBGM_ED) 0.0))

(event EventBeginPlay
  (bind _asmy_hud (Utilities|Casting|CastToMyHUD (HUD|GetHUD (Game|GetPlayerController 0))))
  (bind _output_get (Variables|Default|SetMyHUD _asmy_hud))
  (EventDispatchers|AssignGameStart _output_get (delegate Custom|GameStart_Music))
  (EventDispatchers|AssignBeginMove (Variables|Default|GetMyHUD) (delegate Custom|BeginMove_Music))
  (EventDispatchers|AssignPlayAnimation (Variables|Default|GetMyHUD) (delegate Custom|PlayED)))

(event Collision|EventActorBeginOverlap
  (params (OtherActor :type Actor%20Object%20Reference)))

(event EventTick
  (params (DeltaSeconds :type Float%20%28single-precision%29)))

(fn ConstructionScript)